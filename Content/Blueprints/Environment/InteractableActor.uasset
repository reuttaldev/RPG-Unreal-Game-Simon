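; InteractableActor is an environment actor with a sprite that can flash in a given color, though it contains no interaction logic.
; BeginPlay creates a dynamic material instance on the sprite, then triggers a hardcoded yellow flash after a short delay.
; TriggerFlash takes intensity, color and play rate, then runs a timeline whose alpha scales the material's FlashMultiplier between zero and that intensity.
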(event `self.ReceiveBeginPlay`
  ;[1 1 1] Triggering the event
  (bind _returnvalue (`PrimitiveComponent.CreateDynamicMaterialInstance` (`self.Sprite (Sprite0)`) 0 null "None"))
  (set `self.DynamicSpriteMat` _returnvalue)
  (`KismetSystemLibrary.Delay` 2.0)
  (`self.TriggerFlash` 10.0))

(event `TriggerFlash`
  (params (Multiplier :type "Float (single-precision)" :default 1.0) (Color :type "LinearColor Structure" :default (struct :`R` 1.0 :`G` 0.980559 :`B` 0.164 :`A` 1.0)) (PlayRate :type "Float (single-precision)" :default 5.0))
  ;[1 1 1] Creating the event
  (`MaterialInstanceDynamic.SetScalarParameterValue` (`self.DynamicSpriteMat`) "FlashMultiplier" Multiplier)
  (`MaterialInstanceDynamic.SetVectorParameterValue` (`self.DynamicSpriteMat`) "FlashColor" Color)
  (`TimelineComponent.SetPlayRate` (`self.FlashMultiplier`) PlayRate)
  (bind (_direction _alpha) (`Timeline|FlashMultiplier` :!via `PlayFromStart`)
    (:`Update`
      (`MaterialInstanceDynamic.SetScalarParameterValue` (`self.DynamicSpriteMat`) "FlashMultiplier" (`KismetMathLibrary.Lerp` 0.0 Multiplier _alpha)))))

(fn `UserConstructionScript`)